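; Player controller Blueprint that routes Enhanced Input actions to whichever pawn it possesses.
; On possess it caches the pawn and adds the IMC_PlayerControlls mapping context.
; Move, Look and Jump events forward their values to the pawn as message calls, leaving movement behavior to the pawn.
; Jump sends separate start and stop messages, plus elapsed triggered time while ongoing or triggered.
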(event Input|EnhancedActionEvents|EnhancedInputActionMove
  (params (ActionValue :type Vector%202D%20Structure) (ElapsedSeconds :type Float%20%28double-precision%29) (TriggeredSeconds :type Float%20%28double-precision%29) (InputAction :type Input%20Action%20Object%20Reference :default "/Game/Input/Move.Move"))
  (:Triggered
    (Class|PlayerInputInterface|Move(Message) (Variables|Default|GetPossessed%20Pawn) ActionValue :!label _label))
  (:Started
    (goto _label))
  (:Canceled
    (goto _label))
  (:Completed
    (goto _label)))

(event Input|EnhancedActionEvents|EnhancedInputActionJump
  (params (ActionValue :type Float%20%28double-precision%29) (ElapsedSeconds :type Float%20%28double-precision%29) (TriggeredSeconds :type Float%20%28double-precision%29) (InputAction :type Input%20Action%20Object%20Reference :default "/Game/Input/Jump.Jump"))
  (bind _possessed_pawn (Variables|Default|GetPossessed%20Pawn))
  (:Triggered
    (Character|Jump _possessed_pawn TriggeredSeconds :!label _label))
  (:Started
    (Class|PlayerInputInterface|StartJump(Message) _possessed_pawn))
  (:Ongoing
    (goto _label))
  (:Canceled
    (Class|PlayerInputInterface|StopJump(Message) _possessed_pawn :!label _label_2))
  (:Completed
    (goto _label_2)))

(event Input|EnhancedActionEvents|EnhancedInputActionLook
  (params (ActionValue :type Vector%202D%20Structure) (ElapsedSeconds :type Float%20%28double-precision%29) (TriggeredSeconds :type Float%20%28double-precision%29) (InputAction :type Input%20Action%20Object%20Reference :default "/Game/Input/Look.Look"))
  (Class|PlayerInputInterface|Look(Message) (Variables|Default|GetPossessed%20Pawn) ActionValue))

(event EventPossess
  (params (PossessedPawn :type Pawn%20Object%20Reference))
  (Variables|Default|SetPossessed%20Pawn PossessedPawn)
  (Input|AddMappingContext (PlayerController|LocalPlayerSubsystems|GetEnhancedInputLocalPlayerSubsystem) "/Game/Input/IMC_PlayerControlls.IMC_PlayerControlls" 0 "(bIgnoreAllPressedKeysUntilRelease=True,bForceImmediately=False,bNotifyUserSettings=False)"))

(fn ConstructionScript)